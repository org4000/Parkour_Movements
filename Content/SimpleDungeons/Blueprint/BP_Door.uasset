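; BP_Door is a double dungeon entrance door that swings open and closed as the third-person character passes through its Box trigger.
; When CanOpen is set, begin and end overlap share one FlipFlop that alternates playing and reversing a Timeline.
; The Timeline's curve, scaled by an Angle variable, yaws the two door meshes in opposite directions.
; Open state follows the toggle order rather than which overlap event fired.
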(event OnComponentBeginOverlap(Box)
  (params (OverlappedComponent :type Primitive%20Component%20Object%20Reference) (OtherActor :type Actor%20Object%20Reference) (OtherComp :type Primitive%20Component%20Object%20Reference) (OtherBodyIndex :type Integer) (bFromSweep :type Boolean) (SweepResult :type Hit%20Result%20Structure%20%28by%20ref%29))
  (Utilities|Casting|CastToBP_ThirdPersonCharacter OtherActor)
  (if (Variables|Default|GetCanOpen)
    (Utilities|FlowControl|FlipFlop
      (:A
        (bind _angle (Timeline|Timeline Play)
          (:Update
            (Transformation|SetRelativeRotation (Variables|Default|GetSM_Env_Undead_Entrance_Door_01) (Math|Rotator|MakeRotator 0.0 0.0 (* (* _angle (Variables|Default|GetAngle)) -1.0)) false false)
            (Transformation|SetRelativeRotation (Variables|Default|GetSM_Env_Undead_Entrance_Door_02) (Math|Rotator|MakeRotator 0.0 0.0 (* _angle (Variables|Default|GetAngle))) false false))))
      (:B
        (Timeline|Timeline Reverse)))))

(event OnComponentEndOverlap(Box)
  (params (OverlappedComponent :type Primitive%20Component%20Object%20Reference) (OtherActor :type Actor%20Object%20Reference) (OtherComp :type Primitive%20Component%20Object%20Reference) (OtherBodyIndex :type Integer))
  (Utilities|Casting|CastToBP_ThirdPersonCharacter (stale OnComponentBeginOverlap(Box) OtherActor))
  (if (Variables|Default|GetCanOpen)
    (Utilities|FlowControl|FlipFlop
      (:A
        (bind _angle (Timeline|Timeline Play)
          (:Update
            (Transformation|SetRelativeRotation (Variables|Default|GetSM_Env_Undead_Entrance_Door_01) (Math|Rotator|MakeRotator 0.0 0.0 (* (* _angle (Variables|Default|GetAngle)) -1.0)) false false)
            (Transformation|SetRelativeRotation (Variables|Default|GetSM_Env_Undead_Entrance_Door_02) (Math|Rotator|MakeRotator 0.0 0.0 (* _angle (Variables|Default|GetAngle))) false false))))
      (:B
        (Timeline|Timeline Reverse)))))

(fn ConstructionScript)