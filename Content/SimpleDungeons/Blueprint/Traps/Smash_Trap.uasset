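; Smash Trap is a dungeon hazard that moves repeatedly and damages any actor overlapping its Death component.
; A timeline lerps the Scene component between a Distance offset and its origin, calling Smash again on finish to loop.
; On the first call the timeline starts at once and a DoOnce-gated Delay restarts it later, setting the cycle's phase.
; Overlaps apply a fixed amount of damage.
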(event OnComponentBeginOverlap(Death)
  (params (OverlappedComponent :type Primitive%20Component%20Object%20Reference) (OtherActor :type Actor%20Object%20Reference) (OtherComp :type Primitive%20Component%20Object%20Reference) (OtherBodyIndex :type Integer) (bFromSweep :type Boolean) (SweepResult :type Hit%20Result%20Structure%20%28by%20ref%29))
  (Game|Damage|ApplyDamage OtherActor 1e+01 0 0))

(event Custom|Smash
  (Utilities|FlowControl|Sequence
    (:then_0
      (Utilities|FlowControl|DoOnce false
        (:Completed
          (Utilities|FlowControl|Delay (Variables|Default|GetDelay))
          (bind _smash (Timeline|Timeline PlayFromStart)
            (:Update
              (Transformation|SetRelativeLocation (Variables|Default|GetScene) (Math|Vector|Lerp(Vector) (Variables|Default|GetDistance) "0, 0, 0" _smash) false false))
            (:Finished
              (CallFunction|Smash))))))
    (:then_1
      (Timeline|Timeline PlayFromStart))))

(event EventBeginPlay
  (CallFunction|Smash))

(fn ConstructionScript)